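; Character select display actor that previews each remaining character with its booster mesh and car and bumper materials.
; Left and right scroll events cycle a wrapping index through parallel arrays to update the preview.
; SelectChar records the mesh's visual ID in the game instance for the gamemode's selecting controller, then removes that entry from every array.
; It then resets to the first remaining character, or starts the game when none remain.
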(event Custom|ScrollCharRight
  (bind _characters (Variables|Default|GetCharacters))
  (bind _result (Math|Integer|IncrementInt (Variables|Default|GetCurrentCharID))
    (:%20%20
      (bind _output_get (Variables|Default|SetCurrentCharID (Math|Integer|%(Integer) _result (Utilities|Array|Length _characters))))
      (Components|StaticMesh|SetStaticMesh (Variables|Default|GetMesh) (Utilities|Array|Get(acopy) _characters _output_get))
      (Components|StaticMesh|SetStaticMesh (Variables|Default|GetPole) (Utilities|Array|Get(acopy) (Variables|Default|GetBoosters) (Variables|Default|GetCurrentCharID)))
      ;[0.15 0.15 0.15 0.5] Update Car visuals
      (Rendering|Material|SetMaterial (Variables|Default|GetCar) 0 (Utilities|Array|Get(acopy) (Variables|Default|GetCarMaterials) (Variables|Default|GetCurrentCharID)))
      (Rendering|Material|SetMaterial (Variables|Default|GetCar) 1 (Utilities|Array|Get(acopy) (Variables|Default|GetBumperMaterials) (Variables|Default|GetCurrentCharID))))))

(event Custom|ScrollCharLeft
  (bind _characters (Variables|Default|GetCharacters))
  (bind _result (Math|Integer|DecrementInt (Variables|Default|GetCurrentCharID))
    (:%20%20
      (if (< _result 0)
        (Variables|Default|SetCurrentCharID (- (Utilities|Array|Length _characters) 1)))
      (Components|StaticMesh|SetStaticMesh (Variables|Default|GetMesh) (Utilities|Array|Get(acopy) _characters (Variables|Default|GetCurrentCharID)))
      (Components|StaticMesh|SetStaticMesh (Variables|Default|GetPole) (Utilities|Array|Get(acopy) (Variables|Default|GetBoosters) (Variables|Default|GetCurrentCharID)))
      ;[0.15 0.15 0.15 0.5] Update Car visuals
      (Rendering|Material|SetMaterial (Variables|Default|GetCar) 0 (Utilities|Array|Get(acopy) (Variables|Default|GetCarMaterials) (Variables|Default|GetCurrentCharID)))
      (Rendering|Material|SetMaterial (Variables|Default|GetCar) 1 (Utilities|Array|Get(acopy) (Variables|Default|GetBumperMaterials) (Variables|Default|GetCurrentCharID))))))

(event Custom|SelectChar
  (bind _asbumpurr_cars_game_instance (Utilities|Casting|CastToBumpurrCarsGameInstance (Game|GetGameInstance)))
  (bind _asbp_char_sel_gamemode (Utilities|Casting|CastToBP_CharSelGamemode (Game|GetGameMode)))
  (Class|BumpurrCarsGameInstance|InsertVisualID _asbumpurr_cars_game_instance (Variables|/Game/BumpurrCars/Blueprints/Core/BP_CharSelGamemode.BP_CharSelGamemode_C|GetCurrSelectingID _asbp_char_sel_gamemode) (.Value (Utilities|Map|Find (Variables|Default|GetMeshVisID) (Utilities|Array|Get(acopy) (Variables|Default|GetCharacters) (Variables|Default|GetCurrentCharID)))))
  (Utilities|Array|RemoveIndex (Variables|Default|GetCharacters) (Variables|Default|GetCurrentCharID))
  (Utilities|Array|RemoveIndex (Variables|Default|GetBoosters) (Variables|Default|GetCurrentCharID))
  (Utilities|Array|RemoveIndex (Variables|Default|GetCarMaterials) (Variables|Default|GetCurrentCharID))
  (Utilities|Array|RemoveIndex (Variables|Default|GetBumperMaterials) (Variables|Default|GetCurrentCharID))
  (Variables|Default|SetCurrentCharID 0)
  (if (Utilities|Array|IsEmpty (Variables|Default|GetCharacters))
    (bind _asbp_char_sel_gamemode_2 (Utilities|Casting|CastToBP_CharSelGamemode (Game|GetGameMode)))
    (Default|StartGame _asbp_char_sel_gamemode_2)
    (else
      (Components|StaticMesh|SetStaticMesh (Variables|Default|GetMesh) (Utilities|Array|Get(acopy) (Variables|Default|GetCharacters)))
      (Components|StaticMesh|SetStaticMesh (Variables|Default|GetPole) (Utilities|Array|Get(acopy) (Variables|Default|GetBoosters)))
      ;[0.15 0.15 0.15 0.5] Update Car visuals
      (Rendering|Material|SetMaterial (Variables|Default|GetCar) 0 (Utilities|Array|Get(acopy) (Variables|Default|GetCarMaterials)))
      (Rendering|Material|SetMaterial (Variables|Default|GetCar) 1 (Utilities|Array|Get(acopy) (Variables|Default|GetBumperMaterials))))))

(fn ConstructionScript)