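; BP_CharSelGamemode runs the BumpurrCars character selection screen for local multiplayer.
; On BeginPlay it creates three extra local players, shows WBP_CharSel and focuses it in game-and-UI input with the cursor hidden.
; NextPlayer advances the selecting player ID through 3, moving a looping force feedback rumble to that player's controller to signal their turn.
; StartGame opens the BumpurrCars_P level.
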(event Custom|StartGame
  (Game|OpenLevel(byObjectReference) "/Game/BumpurrCars/Levels/BumpurrCars_P.BumpurrCars_P"))

(event EventBeginPlay
  (bind _returnvalue (Game|GetPlayerController 0))
  (Class|GameplayStatics|CreatePlayer -1)
  (Class|GameplayStatics|CreatePlayer -1)
  (Class|GameplayStatics|CreatePlayer -1)
  (bind _returnvalue_2 (UserInterface|CreateWidget "/Game/BumpurrCars/UI/Widgets/WBP_CharSel.WBP_CharSel_C"))
  (Variables|Default|SetUIWidget _returnvalue_2)
  (UserInterface|Viewport|AddtoViewport _returnvalue_2 0)
  (Variables|/Script/Engine.PlayerController|SetbShowMouseCursor _returnvalue false)
  (Input|SetInputModeGameandUI _returnvalue _returnvalue_2 "DoNotLock" true false))

(event EventTick
  (params (DeltaSeconds :type Float%20%28single-precision%29)))

(fn ConstructionScript)

(fn NextPlayer
  (if (>= (Variables|Default|GetCurrSelectingID) 0)
    (Game|Feedback|ClientStopForceFeedback (Game|GetPlayerController (Variables|Default|GetCurrSelectingID)) "/Game/BumpurrCars/Feedback/Controller/HF_TurnToSelect.HF_TurnToSelect" "None"))
  (bind _result (Math|Integer|IncrementInt (Variables|Default|GetCurrSelectingID))
    (:%20%20
      (bind _output_get (Variables|Default|SetCurrSelectingID _result))
      (if (<= _output_get 3)
        (Game|Feedback|ClientPlayForceFeedback (Game|GetPlayerController _output_get) "/Game/BumpurrCars/Feedback/Controller/HF_TurnToSelect.HF_TurnToSelect" "None" true false false)))))