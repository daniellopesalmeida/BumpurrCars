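; Player controller for the character selection screen that turns left and right selection input into UI navigation.
; On release of SelLeft or SelRight, it casts the game mode to BP_CharSelGamemode and compares its controller ID to CurrSelectingID.
; Only the currently selecting player's input reaches the game mode's UI widget, through LeftClicked or RightClicked.
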(event EventBeginPlay)

(event EventTick
  (params (DeltaSeconds :type Float%20%28single-precision%29)))

(event Input|ActionEvents|InputActionSelLeft
  (params (Key :type Key%20Structure :default "None"))
  (:Released
    (bind _asbp_char_sel_gamemode (Utilities|Casting|CastToBP_CharSelGamemode (Game|GetGameMode)))
    (if (== (Class|GameplayStatics|GetPlayerControllerID self) (Variables|/Game/BumpurrCars/Blueprints/Core/BP_CharSelGamemode.BP_CharSelGamemode_C|GetCurrSelectingID _asbp_char_sel_gamemode))
      (Default|LeftClicked (Variables|/Game/BumpurrCars/Blueprints/Core/BP_CharSelGamemode.BP_CharSelGamemode_C|GetUIWidget _asbp_char_sel_gamemode)))))

(event Input|ActionEvents|InputActionSelRight
  (params (Key :type Key%20Structure :default "None"))
  (:Released
    (bind _asbp_char_sel_gamemode (Utilities|Casting|CastToBP_CharSelGamemode (Game|GetGameMode)))
    (if (== (Class|GameplayStatics|GetPlayerControllerID self) (Variables|/Game/BumpurrCars/Blueprints/Core/BP_CharSelGamemode.BP_CharSelGamemode_C|GetCurrSelectingID _asbp_char_sel_gamemode))
      (Default|RightClicked (Variables|/Game/BumpurrCars/Blueprints/Core/BP_CharSelGamemode.BP_CharSelGamemode_C|GetUIWidget _asbp_char_sel_gamemode)))))

(fn ConstructionScript)